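; BP_Corde2 is a player 2 rope prop that stays invisible until its animation event fires.
; It creates a dynamic opacity material and binds AnimCAS to play the weapon montage with an attached sound.
; The JaugeFeerieDecor gauge on the first BP_SpritesDecor found scales both opacity and volume.
; The rope hides again when the montage completes, and CanCas2 gates replay without being reset here.
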(event `self.ReceiveBeginPlay`
  (add `self.PlayArmesAnims` (delegate `AnimCAS`))
  (bind _returnvalue (`PrimitiveComponent.CreateDynamicMaterialInstance` (`self.Mesh`) 0 "/Game/M_Opacity.M_Opacity" "None"))
  (bind _output_get (set `self.ChiantMaterial` _returnvalue))
  (`MaterialInstanceDynamic.SetScalarParameterValue` _output_get "Opacity" 0.0)
  (bind _outactors (`GameplayStatics.GetAllActorsOfClass` "/Game/ThirdPerson/Blueprints/BP_SpritesDecor.BP_SpritesDecor_C"))
  (bind _asbp_sprites_decor (cast `/Game/ThirdPerson/Blueprints/BP_SpritesDecor` (`|GetArrayItem` _outactors)))
  (set `self.As BP Sprites Decor` _asbp_sprites_decor))

(event `AnimCAS`
  (bind _returnvalue (/ (`KismetMathLibrary.Conv_IntToDouble` (`/Game/ThirdPerson/Blueprints/BP_SpritesDecor.JaugeFeerieDecor` (`self.As BP Sprites Decor`))) 100.0))
  (if (`self.CanCas2`)
    (set `self.CanCas2` false)
    (`MaterialInstanceDynamic.SetScalarParameterValue` (`self.ChiantMaterial`) "Opacity" _returnvalue)
    (set `self.IsRolling` true)
    (`|PlayMontage` (`self.Mesh`) (`self.ArmesMontage`)
      (:`then`
        (`GameplayStatics.SpawnSoundAttached` "/Game/Sounds/CAS2.CAS2" (`self.Mesh`) "None" (0.0 0.0 0.0) (struct) "KeepRelativeOffset" false _returnvalue 1.0 0.0 null null))
      (:`OnCompleted`
        (`MaterialInstanceDynamic.SetScalarParameterValue` (`self.ChiantMaterial`) "Opacity" 0.0)
        (set `self.IsRolling` false)))))

(fn `UserConstructionScript`)