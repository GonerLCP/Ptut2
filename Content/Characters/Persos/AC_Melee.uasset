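; Character component that plays mime action montages for hammer, jump rope and balloon, each with attack, reception ("Recep") and combo versions.
; Shared boolean gates block overlapping moves, while montage notifies open and close combo windows and Hit notifies shake the camera at the first CameraActor.
; Finishing the basic rope or balloon montage enables flags on the matching world actors (BP_Corde/BP_Corde2, BP_Ballon/BallonPose2).
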(event `self.ReceiveBeginPlay`
  (bind _ascharacter (cast `Character` (`self.GetOwner`)))
  (set `self.Owner` _ascharacter)
  (bind _outactors (`GameplayStatics.GetAllActorsOfClass` "/Game/ThirdPerson/Blueprints/BP_SpritesDecor.BP_SpritesDecor_C"))
  (bind _asbp_sprites_decor (cast `/Game/ThirdPerson/Blueprints/BP_SpritesDecor` (`|GetArrayItem` _outactors)))
  (set `self.As BP Sprites Decor` _asbp_sprites_decor))

(event `Attack`
  ;[1 1 1] Hammer
  (if (`self.bCanSimple`)
    (set `self.bCanSimple` false)
    (set `self.bCanSimpleRecep` false)
    (bind _notifyname (`|PlayMontage` (`Character.Mesh` (`self.Owner`)) "/Game/Characters/Persos/Anims/Hammer_Montage.Hammer_Montage")
      (:`OnCompleted`
        (set `self.bCanSimple` true)
        (set `self.bCanSimpleRecep` true))
      (:`OnNotifyBegin`
        (switch `name` _notifyname
          (:`Hit`
            (bind _outactors (`GameplayStatics.GetAllActorsOfClass` "/Script/Engine.CameraActor"))
            (`GameplayStatics.PlayWorldCameraShake` "/Game/Characters/Persos/BP_CameraShake.BP_CameraShake_C" (`Actor.K2_GetActorLocation` (`|GetArrayItem` _outactors)) 0.0 500.0))
          (:`CanCombo`
            (set `self.bCanCombo` true))
          (:`Recovery`
            (set `self.bCanCombo` false)))))))

(event `ComboHammer`
  ;[1 1 1] Hammer
  (if (`self.bCanCombo`)
    (set `self.bCanCombo` false)
    (set `self.bCanSimpleRecep` false)
    (bind _notifyname (`|PlayMontage` (`Character.Mesh` (`self.Owner`)) "/Game/Characters/Persos/Anims/HammerCombo_Montage.HammerCombo_Montage")
      (:`OnCompleted`
        (set `self.bCanSimple` true)
        (set `self.bCanSimpleRecep` true))
      (:`OnNotifyBegin`
        (switch `name` _notifyname
          (:`Hit`
            (bind _outactors (`GameplayStatics.GetAllActorsOfClass` "/Script/Engine.CameraActor"))
            (`GameplayStatics.PlayWorldCameraShake` "/Game/Characters/Persos/BP_CameraShake.BP_CameraShake_C" (`Actor.K2_GetActorLocation` (`|GetArrayItem` _outactors)) 0.0 500.0))
          (:`Recovery`
            (set `self.bCanCombo` false)))))))

(event `Recep Hammer`
  ;[1 1 1] RecepHammer
  (if (`self.bCanSimpleRecep`)
    (set `self.bCanSimpleRecep` false)
    (set `self.bCanSimple` false)
    (set `self.HammerAnimation` true)
    (bind _notifyname (`|PlayMontage` (`Character.Mesh` (`self.Owner`)) "/Game/Characters/Persos/Anims/RecepHammer_Montage.RecepHammer_Montage")
      (:`OnCompleted`
        (set `self.bCanSimpleRecep` true)
        (set `self.bCanSimple` true)
        (set `self.HammerAnimation` false))
      (:`OnNotifyBegin`
        (switch `name` _notifyname
          (:`CanCombo`
            (set `self.bCanComboRecep` true))
          (:`Recovery`
            (set `self.bCanComboRecep` false)))))))

(event `ComboRecepHammer`
  ;[1 1 1] RecepHammer
  (if (`self.bCanComboRecep`)
    (set `self.bCanComboRecep` false)
    (set `self.bCanSimple` false)
    (bind _notifyname (`|PlayMontage` (`Character.Mesh` (`self.Owner`)) "/Game/Characters/Persos/Anims/RecepHammerCombo_Montage.RecepHammerCombo_Montage")
      (:`OnCompleted`
        (set `self.bCanSimpleRecep` true)
        (set `self.bCanSimple` true))
      (:`OnNotifyBegin`
        (switch `name` _notifyname
          (:`Hit`
            (bind _outactors (`GameplayStatics.GetAllActorsOfClass` "/Script/Engine.CameraActor"))
            (`GameplayStatics.PlayWorldCameraShake` "/Game/Characters/Persos/BP_CameraShake.BP_CameraShake_C" (`Actor.K2_GetActorLocation` (`|GetArrayItem` _outactors)) 0.0 500.0))
          (:`Recovery`
            (set `self.bCanSimpleRecep` false)))))))

(event `CordeASauter`
  ;[1 1 1] Cas
  (if (`self.bCanSimple`)
    (set `self.bCanSimple` false)
    (set `self.bCanSimpleRecep` false)
    (bind _notifyname (`|PlayMontage` (`Character.Mesh` (`self.Owner`)) "/Game/Characters/Persos/Anims/CordeASauter_Montage.CordeASauter_Montage")
      (:`OnCompleted`
        (set `self.bCanSimple` true)
        (set `self.bCanSimpleRecep` true)
        (bind _outactors (`GameplayStatics.GetAllActorsOfClass` "/Game/Characters/Persos/Armes/Armes/BP_Corde.BP_Corde_C"))
        (set `/Game/Characters/Persos/Armes/Armes/BP_Corde.CanCas` true (`|GetArrayItem` _outactors))
        (bind _outactors_2 (`GameplayStatics.GetAllActorsOfClass` "/Game/Characters/Persos/ArmesPlayer2/BP_Corde2.BP_Corde2_C"))
        (set `/Game/Characters/Persos/ArmesPlayer2/BP_Corde2.CanCas2` true (`|GetArrayItem` _outactors_2)))
      (:`OnNotifyBegin`
        (switch `name` _notifyname
          (:`CanCombo`
            (set `self.bCanCombo` true))
          (:`Recovery`
            (set `self.bCanCombo` false)))))))

(event `ComboCordeASauter`
  ;[1 1 1] Cas
  (if (`self.bCanCombo`)
    (set `self.bCanCombo` false)
    (set `self.bCanSimple` false)
    (bind _notifyname (`|PlayMontage` (`Character.Mesh` (`self.Owner`)) "/Game/Characters/Persos/Anims/CordeASauterCombo_Montage.CordeASauterCombo_Montage")
      (:`OnCompleted`
        (set `self.bCanSimple` true)
        (set `self.bCanSimpleRecep` true))
      (:`OnNotifyBegin`
        (switch `name` _notifyname
          (:`Recovery`
            (set `self.bCanSimpleRecep` false)))))))

(event `RecepCAS`
  ;[1 1 1] RecepCAS
  (if (`self.bCanSimpleRecep`)
    (set `self.bCanSimpleRecep` false)
    (set `self.bCanSimple` false)
    (set `self.CASAnimation` true)
    (bind _notifyname (`|PlayMontage` (`Character.Mesh` (`self.Owner`)) "/Game/Characters/Persos/Anims/RecepCordeASauter_Montage.RecepCordeASauter_Montage")
      (:`OnCompleted`
        (set `self.bCanSimpleRecep` true)
        (set `self.bCanSimple` true)
        (set `self.CASAnimation` false))
      (:`OnNotifyBegin`
        (switch `name` _notifyname
          (:`Hit`
            (bind _outactors (`GameplayStatics.GetAllActorsOfClass` "/Script/Engine.CameraActor"))
            (`GameplayStatics.PlayWorldCameraShake` "/Game/Characters/Persos/BP_CameraShake.BP_CameraShake_C" (`Actor.K2_GetActorLocation` (`|GetArrayItem` _outactors)) 0.0 500.0))
          (:`CanCombo`
            (set `self.bCanComboRecep` true))
          (:`Recovery`
            (set `self.bCanComboRecep` false)))))))

(event `ComboRecepCas`
  ;[1 1 1] RecepCAS
  (if (`self.bCanComboRecep`)
    (set `self.bCanComboRecep` false)
    (set `self.bCanSimple` false)
    (bind _notifyname (`|PlayMontage` (`Character.Mesh` (`self.Owner`)) "/Game/Characters/Persos/Anims/ReceptionCordeASauterCombo_Montage.ReceptionCordeASauterCombo_Montage")
      (:`OnCompleted`
        (set `self.bCanSimpleRecep` true)
        (set `self.bCanSimple` true))
      (:`OnNotifyBegin`
        (switch `name` _notifyname
          (:`Hit`
            (bind _outactors (`GameplayStatics.GetAllActorsOfClass` "/Script/Engine.CameraActor"))
            (`GameplayStatics.PlayWorldCameraShake` "/Game/Characters/Persos/BP_CameraShake.BP_CameraShake_C" (`Actor.K2_GetActorLocation` (`|GetArrayItem` _outactors)) 0.0 500.0))
          (:`Recovery`
            (set `self.bCanSimpleRecep` false)))))))

(event `Ballon`
  ;[1 1 1] Ballon
  (if (`self.bCanSimple`)
    (set `self.bCanSimple` false)
    (set `self.bCanSimpleRecep` false)
    (bind _notifyname (`|PlayMontage` (`Character.Mesh` (`self.Owner`)) "/Game/Characters/Persos/Anims/MimeBallon_Anim_Montage.MimeBallon_Anim_Montage")
      (:`OnCompleted`
        (set `self.bCanSimple` true)
        (set `self.bCanSimpleRecep` true)
        (bind _outactors (`GameplayStatics.GetAllActorsOfClass` "/Game/Characters/Persos/Armes/Balle/CorrectionDuBallon/Ballon1/BP_Ballon.BP_Ballon_C"))
        (set `/Game/Characters/Persos/Armes/Balle/CorrectionDuBallon/Ballon1/BP_Ballon.CanShoot` true (`|GetArrayItem` _outactors))
        (bind _outactors_2 (`GameplayStatics.GetAllActorsOfClass` "/Game/Characters/Persos/ArmesPlayer2/Balle2/BallonPose2.BallonPose2_C"))
        (set `/Game/Characters/Persos/ArmesPlayer2/Balle2/BallonPose2.CanShoot2` true (`|GetArrayItem` _outactors_2)))
      (:`OnNotifyBegin`
        (switch `name` _notifyname
          (:`CanCombo`
            (set `self.bCanCombo` true))
          (:`Recovery`
            (set `self.bCanCombo` false)))))))

(event `ComboBallon`
  ;[1 1 1] Ballon
  (if (`self.bCanCombo`)
    (set `self.bCanCombo` false)
    (set `self.bCanSimple` false)
    (bind _notifyname (`|PlayMontage` (`Character.Mesh` (`self.Owner`)) "/Game/Characters/Persos/Anims/MimeLancePierre_Anim_Montage.MimeLancePierre_Anim_Montage")
      (:`OnCompleted`
        (set `self.bCanSimple` true)
        (set `self.bCanSimpleRecep` true))
      (:`OnNotifyBegin`
        (switch `name` _notifyname
          (:`Hit`
            (bind _outactors (`GameplayStatics.GetAllActorsOfClass` "/Script/Engine.CameraActor"))
            (`GameplayStatics.PlayWorldCameraShake` "/Game/Characters/Persos/BP_CameraShake.BP_CameraShake_C" (`Actor.K2_GetActorLocation` (`|GetArrayItem` _outactors)) 0.0 500.0))
          (:`Recovery`
            (set `self.bCanSimpleRecep` false)))))))

(event `RecepBallon`
  ;[1 1 1] RecepBallon
  (if (`self.bCanSimpleRecep`)
    (set `self.bCanSimpleRecep` false)
    (set `self.bCanSimple` false)
    (bind _notifyname (`|PlayMontage` (`Character.Mesh` (`self.Owner`)) "/Game/Characters/Persos/Anims/MimeRecepBallon_Anim_Montage.MimeRecepBallon_Anim_Montage")
      (:`OnCompleted`
        (set `self.bCanSimpleRecep` true)
        (set `self.bCanSimple` true))
      (:`OnNotifyBegin`
        (switch `name` _notifyname
          (:`Hit`
            (bind _outactors (`GameplayStatics.GetAllActorsOfClass` "/Script/Engine.CameraActor"))
            (`GameplayStatics.PlayWorldCameraShake` "/Game/Characters/Persos/BP_CameraShake.BP_CameraShake_C" (`Actor.K2_GetActorLocation` (`|GetArrayItem` _outactors)) 0.0 500.0))
          (:`CanCombo`
            (set `self.bCanComboRecep` true))
          (:`Recovery`
            (set `self.bCanComboRecep` false)))))))

(event `ComboRecepBallon`
  ;[1 1 1] RecepBallon
  (if (`self.bCanComboRecep`)
    (set `self.bCanComboRecep` false)
    (set `self.bCanSimple` false)
    (bind _notifyname (`|PlayMontage` (`Character.Mesh` (`self.Owner`)) "/Game/Characters/Persos/Anims/MimeRecepLancePierre_Anim_Montage.MimeRecepLancePierre_Anim_Montage")
      (:`OnCompleted`
        (set `self.bCanSimpleRecep` true)
        (set `self.bCanSimple` true))
      (:`OnNotifyBegin`
        (switch `name` _notifyname
          (:`Hit`
            (bind _outactors (`GameplayStatics.GetAllActorsOfClass` "/Script/Engine.CameraActor"))
            (`GameplayStatics.PlayWorldCameraShake` "/Game/Characters/Persos/BP_CameraShake.BP_CameraShake_C" (`Actor.K2_GetActorLocation` (`|GetArrayItem` _outactors)) 0.0 500.0))
          (:`Recovery`
            (set `self.bCanSimpleRecep` false)))))))