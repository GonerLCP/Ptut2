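; MarteauBP is a hammer weapon Blueprint that shows the hammer only while its swing animation plays.
; On BeginPlay it hides the Marteau mesh and binds AnimHammer to the PlayHammerAnim event.
; AnimHammer, gated by CanHammer to block overlapping swings, reveals the mesh and plays the montage, then hides it and re-arms on completion.
; The montage's "Can Combo" notify only triggers the attached hammer sound.
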(event `self.ReceiveBeginPlay`
  (`SceneComponent.SetVisibility` (`self.Marteau`) false false)
  (add `self.PlayHammerAnim` (delegate `AnimHammer`)))

(event `AnimHammer`
  (if (`self.CanHammer`)
    (set `self.CanHammer` false)
    (`SceneComponent.SetVisibility` (`self.Marteau`) true false)
    (bind _notifyname (`|PlayMontage` (`self.Marteau`) (`self.HammerMontage`))
      (:`OnCompleted`
        (`SceneComponent.SetVisibility` (`self.Marteau`) false false)
        (set `self.CanHammer` true))
      (:`OnNotifyBegin`
        (switch `name` _notifyname
          (:`CanCombo`
            (`GameplayStatics.SpawnSoundAttached` "/Game/Sounds/Marteau.Marteau" (`self.Marteau`) "None" (0.0 0.0 0.0) (struct) "KeepRelativeOffset" false 1.0 1.0 0.0 null null)))))))

(fn `UserConstructionScript`)