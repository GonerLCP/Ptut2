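; BP_BallonShoot is a weapon balloon actor that shows an animation when its BallePosée event fires, then destroys itself.
; At BeginPlay it creates a dynamic opacity material on the balloon mesh, hides it, and caches the level's BP_SpritesDecor.
; BallePosée sets opacity from that actor's JaugeFeerieDecor gauge scaled down by 100, plays the DernièreChance montage, and destroys the actor on completion.
; A leftover F key handler prints a debug string.
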(event `self.ReceiveBeginPlay`
  (bind _returnvalue (`PrimitiveComponent.CreateDynamicMaterialInstance` (`self.ElBallon1`) 0 "/Game/M_Opacity.M_Opacity" "None"))
  (bind _output_get (set `self.Material` _returnvalue))
  (`MaterialInstanceDynamic.SetScalarParameterValue` _output_get "Opacity" 0.0)
  (bind _outactors (`GameplayStatics.GetAllActorsOfClass` "/Game/ThirdPerson/Blueprints/BP_SpritesDecor.BP_SpritesDecor_C"))
  (bind _asbp_sprites_decor (cast `/Game/ThirdPerson/Blueprints/BP_SpritesDecor` (`|GetArrayItem` _outactors)))
  (set `self.As BP Sprites Decor` _asbp_sprites_decor))

(event `BallePosée`
  (`MaterialInstanceDynamic.SetScalarParameterValue` (`self.Material`) "Opacity" (/ (`KismetMathLibrary.Conv_IntToDouble` (`/Game/ThirdPerson/Blueprints/BP_SpritesDecor.JaugeFeerieDecor` (`self.As BP Sprites Decor`))) 100.0))
  (`|PlayMontage` (`self.ElBallon1`) (`self.DernièreChance`)
    (:`OnCompleted`
      (`self.K2_DestroyActor`))))

(event `Key|F`
  (params (Key :type "Key Structure"))
  (:`Pressed`
    (`KismetSystemLibrary.PrintString` "Hello")))

(fn `UserConstructionScript`)