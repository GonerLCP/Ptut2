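; BP_Marteau is a hammer weapon that plays a swing montage when the PlayHammerAnim event fires, with a flag blocking re-triggers until completion.
; On BeginPlay it creates a dynamic steel material with zero Opacity and caches the first BP_SpritesDecor actor.
; Each swing sets Opacity from that actor's JaugeFeerieDecor gauge, resetting it on completion.
; The montage's notify plays an attached hammer sound with volume scaled by the same gauge.
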(event `self.ReceiveBeginPlay`
  (add `self.PlayHammerAnim` (delegate `AnimHammer`))
  (bind _returnvalue (`PrimitiveComponent.CreateDynamicMaterialInstance` (`self.Marteau`) 0 "/Game/M_Opa_Metal_Steel.M_Opa_Metal_Steel" "None"))
  (bind _output_get (set `self.WoodMaterial` _returnvalue))
  (`MaterialInstanceDynamic.SetScalarParameterValue` _output_get "Opacity" 0.0)
  (bind _outactors (`GameplayStatics.GetAllActorsOfClass` "/Game/ThirdPerson/Blueprints/BP_SpritesDecor.BP_SpritesDecor_C"))
  (bind _asbp_sprites_decor (cast `/Game/ThirdPerson/Blueprints/BP_SpritesDecor` (`|GetArrayItem` _outactors)))
  (set `self.As BP Sprites Decor` _asbp_sprites_decor))

(event `AnimHammer`
  (bind _returnvalue (/ (`KismetMathLibrary.Conv_IntToDouble` (`/Game/ThirdPerson/Blueprints/BP_SpritesDecor.JaugeFeerieDecor` (`self.As BP Sprites Decor`))) 100.0))
  (if (`self.CanHammer`)
    (set `self.CanHammer` false)
    (`MaterialInstanceDynamic.SetScalarParameterValue` (`self.WoodMaterial`) "Opacity" _returnvalue)
    (bind _notifyname (`|PlayMontage` (`self.Marteau`) (`self.HammerMontage`))
      (:`OnCompleted`
        (`MaterialInstanceDynamic.SetScalarParameterValue` (`self.WoodMaterial`) "Opacity" 0.0)
        (set `self.CanHammer` true))
      (:`OnNotifyBegin`
        (switch `name` _notifyname
          (:`CanCombo`
            (`GameplayStatics.SpawnSoundAttached` "/Game/Sounds/Marteau.Marteau" (`self.Marteau`) "None" (0.0 0.0 0.0) (struct) "KeepRelativeOffset" false _returnvalue 1.0 0.0 null null)))))))

(fn `UserConstructionScript`)