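; BP_BallonPose is a balloon weapon actor that plays the balloon's shooting animation when the bound AnimBallon event fires.
; A dynamic opacity material keeps it invisible until then, with visibility scaled by the JaugeFeerieDecor gauge from BP_SpritesDecor.
; AnimBallon clears CanShoot, plays a montage with attached sound, then on completion hides the balloon and calls ShootBalon on the player character.
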(event `self.ReceiveBeginPlay`
  (add `self.PlayBallonAnim` (delegate `AnimBallon`))
  (bind _returnvalue (`PrimitiveComponent.CreateDynamicMaterialInstance` (`self.ElBallon`) 0 "/Game/M_Opacity.M_Opacity" "None"))
  (bind _output_get (set `self.BallonMaterial` _returnvalue))
  (`MaterialInstanceDynamic.SetScalarParameterValue` _output_get "Opacity" 0.0)
  (bind _outactors (`GameplayStatics.GetAllActorsOfClass` "/Game/ThirdPerson/Blueprints/BP_SpritesDecor.BP_SpritesDecor_C"))
  (bind _asbp_sprites_decor (cast `/Game/ThirdPerson/Blueprints/BP_SpritesDecor` (`|GetArrayItem` _outactors)))
  (set `self.As BP Sprites Decor` _asbp_sprites_decor))

(event `AnimBallon`
  (if (`self.CanShoot`)
    (set `self.CanShoot` false)
    (`MaterialInstanceDynamic.SetScalarParameterValue` (`self.BallonMaterial`) "Opacity" (/ (`KismetMathLibrary.Conv_IntToDouble` (`/Game/ThirdPerson/Blueprints/BP_SpritesDecor.JaugeFeerieDecor` (`self.As BP Sprites Decor`))) 100.0))
    (set `self.IsShooting` true)
    (`|PlayMontage` (`self.ElBallon`) (`self.BallonMontage`)
      (:`then`
        (`GameplayStatics.SpawnSoundAttached` null (`self.ElBallon`) "None" (0.0 0.0 0.0) (struct) "KeepRelativeOffset" false 1.0 1.0 0.0 null null))
      (:`OnCompleted`
        (`MaterialInstanceDynamic.SetScalarParameterValue` (`self.BallonMaterial`) "Opacity" 0.0)
        (set `self.IsShooting` false)
        (bind _outactors (`GameplayStatics.GetAllActorsOfClass` "/Game/ThirdPerson/Blueprints/BP_ThirdPersonCharacter.BP_ThirdPersonCharacter_C"))
        (`/Game/ThirdPerson/Blueprints/BP_ThirdPersonCharacter.ShootBalon` (`|GetArrayItem` _outactors))))))

(fn `UserConstructionScript`)