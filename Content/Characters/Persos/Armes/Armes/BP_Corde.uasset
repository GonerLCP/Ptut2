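; Rope weapon Blueprint that appears only while its montage plays, triggered through the PlayArmesAnims event.
; At BeginPlay it creates a dynamic opacity material, hides the mesh and caches the first BP_SpritesDecor in the level.
; AnimCAS, gated by CanCas, sets opacity from that actor's fairy gauge (JaugeFeerieDecor), flags IsRolling and plays the montage.
; On completion it hides the rope and clears IsRolling; CanCas is not re-enabled here.
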(event `self.ReceiveBeginPlay`
  (add `self.PlayArmesAnims` (delegate `AnimCAS`))
  (bind _returnvalue (`PrimitiveComponent.CreateDynamicMaterialInstance` (`self.Mesh`) 0 "/Game/M_Opacity.M_Opacity" "None"))
  (bind _output_get (set `self.ChiantMaterial` _returnvalue))
  (`MaterialInstanceDynamic.SetScalarParameterValue` _output_get "Opacity" 0.0)
  (bind _outactors (`GameplayStatics.GetAllActorsOfClass` "/Game/ThirdPerson/Blueprints/BP_SpritesDecor.BP_SpritesDecor_C"))
  (bind _asbp_sprites_decor (cast `/Game/ThirdPerson/Blueprints/BP_SpritesDecor` (`|GetArrayItem` _outactors)))
  (set `self.As BP Sprites Decor` _asbp_sprites_decor))

(event `AnimCAS`
  (if (`self.CanCas`)
    (set `self.CanCas` false)
    (`MaterialInstanceDynamic.SetScalarParameterValue` (`self.ChiantMaterial`) "Opacity" (/ (`KismetMathLibrary.Conv_IntToDouble` (`/Game/ThirdPerson/Blueprints/BP_SpritesDecor.JaugeFeerieDecor` (`self.As BP Sprites Decor`))) 100.0))
    (set `self.IsRolling` true)
    (bind _notifyname (`|PlayMontage` (`self.Mesh`) (`self.ArmesMontage`))
      (:`OnCompleted`
        (`MaterialInstanceDynamic.SetScalarParameterValue` (`self.ChiantMaterial`) "Opacity" 0.0)
        (set `self.IsRolling` false))
      (:`OnNotifyBegin`
        (switch `name` _notifyname)))))

(fn `UserConstructionScript`)