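; BP_BallonTest is a balloon actor, filed under character weapon projectiles, that plays a one-time shot animation and then destroys itself.
; On BeginPlay it hides its MouvementBallon mesh through a dynamic opacity material, binds to an animation dispatcher and caches the first BP_SpritesDecor.
; When the dispatcher fires and shooting is allowed, opacity follows the decor's fairy gauge percentage while ArmesMontage plays.
; Montage completion hides the mesh and destroys the actor.
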(event `self.ReceiveBeginPlay`
  (add `self.AnimBallonDispatcher` (delegate `CallAnimBallon`))
  (bind _returnvalue (`PrimitiveComponent.CreateDynamicMaterialInstance` (`self.MouvementBallon`) 0 "/Game/M_Opacity.M_Opacity" "None"))
  (bind _output_get (set `self.ChiantMaterial` _returnvalue))
  (`MaterialInstanceDynamic.SetScalarParameterValue` _output_get "Opacity" 0.0)
  (bind _outactors (`GameplayStatics.GetAllActorsOfClass` "/Game/ThirdPerson/Blueprints/BP_SpritesDecor.BP_SpritesDecor_C"))
  (bind _asbp_sprites_decor (cast `/Game/ThirdPerson/Blueprints/BP_SpritesDecor` (`|GetArrayItem` _outactors)))
  (set `self.As BP Sprites Decor` _asbp_sprites_decor))

(event `CallAnimBallon`
  (if (`self.CanShoot`)
    (set `self.CanShoot` false)
    (`MaterialInstanceDynamic.SetScalarParameterValue` (`self.ChiantMaterial`) "Opacity" (/ (`KismetMathLibrary.Conv_IntToDouble` (`/Game/ThirdPerson/Blueprints/BP_SpritesDecor.JaugeFeerieDecor` (`self.As BP Sprites Decor`))) 100.0))
    (set `self.IsShooting` true)
    (`|PlayMontage` (`self.MouvementBallon`) (`self.ArmesMontage`)
      (:`OnCompleted`
        (`MaterialInstanceDynamic.SetScalarParameterValue` (`self.ChiantMaterial`) "Opacity" 0.0)
        (set `self.IsShooting` false)
        (`self.K2_DestroyActor`)))))

(fn `UserConstructionScript`)